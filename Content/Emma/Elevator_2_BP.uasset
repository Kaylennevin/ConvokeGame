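; Elevator actor that the third-person character moves between two points by key press.
; Overlapping its Box enables player input on the actor, and leaving the Box disables it.
; J plays the Elevate timeline, which lerps the Elevator component's relative location from StartPoint to EndPoint, and M reverses it.
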(event OnComponentBeginOverlap(Box)
  (params (OverlappedComponent :type Primitive%20Component%20Object%20Reference) (OtherActor :type Actor%20Object%20Reference) (OtherComp :type Primitive%20Component%20Object%20Reference) (OtherBodyIndex :type Integer) (bFromSweep :type Boolean) (SweepResult :type Hit%20Result%20Structure%20%28by%20ref%29))
  (Utilities|Casting|CastToThirdPersonCharacter OtherActor)
  (Input|EnableInput (Game|GetPlayerController 0)))

(event OnComponentEndOverlap(Box)
  (params (OverlappedComponent :type Primitive%20Component%20Object%20Reference) (OtherActor :type Actor%20Object%20Reference) (OtherComp :type Primitive%20Component%20Object%20Reference) (OtherBodyIndex :type Integer))
  (Utilities|Casting|CastToThirdPersonCharacter OtherActor)
  (Input|DisableInput (Game|GetPlayerController 0)))

(event Input|KeyboardEvents|J
  (params (Key :type Key%20Structure :default "None"))
  (:Pressed
    (bind _newtrack_0 (Timeline|Elevate Play)
      (:Update
        (Transformation|SetRelativeLocation (Variables|Default|GetElevator) (Math|Vector|Lerp(Vector) (Variables|Default|GetStart%20Point) (Variables|Default|GetEnd%20Point) _newtrack_0) false false)))))

(event Input|KeyboardEvents|M
  (params (Key :type Key%20Structure :default "None"))
  (:Pressed
    (bind _newtrack_0 (Timeline|Elevate Reverse)
      (:Update
        (Transformation|SetRelativeLocation (Variables|Default|GetElevator) (Math|Vector|Lerp(Vector) (Variables|Default|GetStart%20Point) (Variables|Default|GetEnd%20Point) _newtrack_0) false false)))))

(fn ConstructionScript)