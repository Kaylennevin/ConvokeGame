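; Root bridge actor that grows when the puzzle end fires its move-bridge event, with a camera cutaway to show it.
; BeginPlay binds MoveBridge to the first BP_PuzzleEnd in the level.
; A CameraMove timeline blends the view to BridgeCamera and, on each update, plays a second timeline that stretches the mesh cumulatively along Y scale.
; When growth finishes, a short delay precedes returning the view to PlayerRef.
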(event Custom|MoveBridge
  (bind _mesh (Variables|Default|GetMesh))
  (bind _returnvalue (Transformation|GetWorldScale _mesh))
  (Timeline|CameraMove Play
    (:Update
      (Game|Player|SetViewTargetwithBlend (Game|GetPlayerController 0) (Variables|Default|GetBridgeCamera) 3.0 "VTBlend_Cubic" 0.0 false)
      (bind _distance (Timeline|Timeline_0 Play)
        (:Update
          (Transformation|SetWorldScale3D (Variables|Default|GetMesh) (Math|Vector|MakeVector (.x _returnvalue) (Math|Float|Lerp (.y _returnvalue) (+ (.y _returnvalue) 0.035) _distance) (.z _returnvalue))))
        (:Finished
          (Utilities|FlowControl|Delay 1.0)
          (Game|Player|SetViewTargetwithBlend (Game|GetPlayerController 0) (Variables|Default|GetPlayerRef) 0.0 "VTBlend_Linear" 0.0 false))))))

(event EventBeginPlay
  (bind _outactors (Actor|GetAllActorsOfClass "/Game/Kaylen/BP_PuzzleEnd.BP_PuzzleEnd_C"))
  (Variables|Default|SetPuzzleZoneRef (Utilities|Array|Get(acopy) _outactors))
  (EventDispatchers|BindEventtoMoveBridge (Variables|Default|GetPuzzleZoneRef) (delegate Custom|MoveBridge)))

(fn ConstructionScript)

(fn MoveGameActor
  (return 0))