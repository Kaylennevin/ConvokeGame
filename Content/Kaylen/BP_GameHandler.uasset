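; BP_GameHandler is a game handler Blueprint that changes the look of the level's trees shortly after play begins.
; After a brief delay on BeginPlay, RestoreEnvironment finds actors tagged "Tree" and casts each to BP_Tree.
; Despite the function's name, it gives each tree a wasteland static mesh and a brown material.
; MoveGameActor is an empty stub.
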(event EventBeginPlay
  (Utilities|FlowControl|Delay 2.0)
  (CallFunction|RestoreEnvironment))

(fn ConstructionScript)

(fn RestoreEnvironment
  (bind _outactors (Actor|GetAllActorswithTag "Tree"))
  (for _array_element _outactors
    (bind _asbp_tree (Utilities|Casting|CastToBP_Tree _array_element))
    (Components|StaticMesh|SetStaticMesh (Variables|/Game/Kaylen/Environment/BP_Tree.BP_Tree_C|GetMesh _asbp_tree) "/Game/Kaylen/Environment/Wasteland/tree_wasteland_01.tree_wasteland_01")
    (Rendering|Material|SetMaterial (Variables|/Game/Kaylen/Environment/BP_Tree.BP_Tree_C|GetMesh _asbp_tree) 0 "/Game/Kaylen/CurvedWorld/M_CurvedBRown.M_CurvedBRown")))

(fn MoveGameActor
  (return 0))