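; Puzzle-end actor where three tagged fragments are placed to trigger a bridge event.
; Pressing K reads the tags of the giant's first attached actor; if player and fragment overlap the matching zone, it snaps the artifact to that slot, detaches and locks it.
; A looping timer watches the placed count and fires CallMoveBridge once at three.
; Tick's hologram material switch uses a constant 0, so only the first sphere gets highlighted.
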(event Custom|Bridge
  (if (== (Variables|Default|GetFragmentsPlaced) 3)
    (Development|PrintString "ALL FRAGMENTS PLACE!! PLAY INTENSE SCENE OF BRIDGE BEING BUILT")
    (Utilities|FlowControl|Delay 0.5)
    (Default|CallMoveBridge)
    (Variables|Default|SetFragmentsPlaced 4)))

(event EventTick
  (params (DeltaSeconds :type Float%20%28single-precision%29))
  (Utilities|FlowControl|Delay 1.0)
  (switch int 0
    (:0
      (Rendering|Material|SetMaterial (Variables|Default|GetSphere) 0 "/Game/Kaylen/Shaders/M_Holo.M_Holo"))
    (:1
      (Rendering|Material|SetMaterial (Variables|Default|GetSphere1) 0 "/Game/Kaylen/Shaders/M_Holo.M_Holo")
      (Rendering|Material|SetMaterial (Variables|Default|GetSphere) 0 "/Game/Kaylen/CurvedWorld/M_testartifacts.M_testartifacts"))
    (:2
      (Rendering|Material|SetMaterial (Variables|Default|GetSphere2) 0 "/Game/Kaylen/Shaders/M_Holo.M_Holo")
      (Rendering|Material|SetMaterial (Variables|Default|GetSphere1) 0 "/Game/Kaylen/CurvedWorld/M_testartifacts.M_testartifacts"))
    (:3
      (Rendering|Material|SetMaterial (Variables|Default|GetSphere2) 0 "/Game/Kaylen/CurvedWorld/M_testartifacts.M_testartifacts"))))

(event EventBeginPlay
  (bind _asthird_person_character (Utilities|Casting|CastToThirdPersonCharacter (Game|GetPlayerCharacter 0)))
  (Variables|Default|SetPlayerRef _asthird_person_character)
  (Utilities|Time|SetTimerbyEvent (delegate Custom|Bridge) 0.5 true))

(event Input|KeyboardEvents|K
  (params (Key :type Key%20Structure :default "None"))
  (:Pressed
    (CallFunction|GetAttachedFragment)))

(fn ConstructionScript)

(fn GetAttachedFragment
  (bind _asbp_giant (Utilities|Casting|CastToBP_Giant (Variables|Default|GetGiantRef)))
  (bind _output_get (Variables|Default|SetAttachedActors (Actor|GetAttachedActors _asbp_giant true)))
  (for _array_element (Variables|/Script/Engine.Actor|GetTags (Utilities|Array|Get(acopy) _output_get))
    _)
  (switch name _array_element
    (:Frag1
      (CallFunction|PlaceAttachedFragment (Variables|Default|GetFragmentZone1) (Variables|Default|GetFrag1)))
    (:Frag2
      (CallFunction|PlaceAttachedFragment (Variables|Default|GetFragmentZone2) (Variables|Default|GetSphere2)))
    (:Frag3
      (CallFunction|PlaceAttachedFragment (Variables|Default|GetFragmentZone3) (Variables|Default|GetSphere1)))))

(fn PlaceAttachedFragment
  (params (FragmentZone :type Sphere%20Component%20Object%20Reference) (PlacementMesh :type Static%20Mesh%20Component%20Object%20Reference))
  (bind _returnvalue (Transformation|GetWorldTransform PlacementMesh))
  (if (and (Class|PrimitiveComponent|IsOverlappingComponent (Variables|/Script/Engine.Character|GetCapsuleComponent (Variables|Default|GetPlayerRef)) FragmentZone) (Collision|IsOverlappingActor FragmentZone (Utilities|Array|Get(acopy) (Variables|Default|GetAttachedActors)) :!class /Script/Engine.PrimitiveComponent))
    (bind _asbp_artifact (Utilities|Casting|CastToBP_Artifact (Utilities|Array|Get(acopy) (Variables|Default|GetAttachedActors))))
    (Transformation|SetActorTransform _asbp_artifact (Math|Transform|MakeTransform (.location _returnvalue) (.rotation _returnvalue) (Transformation|GetActorScale3D _asbp_artifact)))
    (Transformation|DetachFromActor _asbp_artifact "KeepWorld" "KeepWorld" "KeepWorld")
    (Variables|/Game/Kaylen/BP_Artifact.BP_Artifact_C|SetCantBeMoved _asbp_artifact true)
    (bind _result (Math|Integer|IncrementInt (Variables|Default|GetFragmentsPlaced))
      (:%20%20
        (Development|PrintString (Utilities|String|Append "fragments placed " (Utilities|String|ToString(Integer) _result)) true true "(R=1.000000,G=0.414395,B=0.000000,A=1.000000)" 5.0)))))

(fn MoveGameActor
  (return 0))