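; BP_Giant is a giant with a happiness meter that also handles interaction prompts for nearby artifacts.
; On BeginPlay it creates the HUD and caches "Fragment"-tagged actors.
; Each tick, while Zone 1 is unrestored, it drains clamped happiness and refreshes the HUD bar.
; Capsule overlap with a BP_Artifact enables interaction if the player's hands are empty, showing WBP_Interact for movable artifacts; ending overlap removes the prompt.
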(event OnComponentBeginOverlap(CapsuleComponent)
  (params (OverlappedComponent :type Primitive%20Component%20Object%20Reference) (OtherActor :type Actor%20Object%20Reference) (OtherComp :type Primitive%20Component%20Object%20Reference) (OtherBodyIndex :type Integer) (bFromSweep :type Boolean) (SweepResult :type Hit%20Result%20Structure%20%28by%20ref%29))
  (bind _asbp_artifact (Utilities|Casting|CastToBP_Artifact OtherActor))
  (if (not (Variables|/Game/ThirdPersonBP/Blueprints/ThirdPersonCharacter.ThirdPersonCharacter_C|GetIsHolding (Variables|Default|GetPlayerRef)))
    (Variables|Default|SetEndOverlap false)
    (if (not (Variables|Default|GetEndOverlap))
      (if (not (Variables|/Game/ThirdPersonBP/Blueprints/ThirdPersonCharacter.ThirdPersonCharacter_C|GetIsHolding (Variables|Default|GetPlayerRef)))
        (Variables|Default|SetCanInteract true)
        (if (not (Variables|/Game/Kaylen/BP_Artifact.BP_Artifact_C|GetCantBeMoved _asbp_artifact))
          (bind _returnvalue (UserInterface|CreateWidget "/Game/Kaylen/UIElements/WBP_Interact.WBP_Interact_C"))
          (bind _output_get (Variables|Default|SetInteractRef _returnvalue))
          (UserInterface|Viewport|AddtoViewport _output_get 0))))))

(event OnComponentEndOverlap(CapsuleComponent)
  (params (OverlappedComponent :type Primitive%20Component%20Object%20Reference) (OtherActor :type Actor%20Object%20Reference) (OtherComp :type Primitive%20Component%20Object%20Reference) (OtherBodyIndex :type Integer))
  (Utilities|Casting|CastToBP_Artifact OtherActor)
  (Variables|Default|SetEndOverlap true)
  (bind _foundwidgets (Widget|GetAllWidgetsOfClass "/Game/Kaylen/UIElements/WBP_Interact.WBP_Interact_C" false))
  (Widget|RemovefromParent _foundwidgets))

(event EventTick
  (params (DeltaSeconds :type Float%20%28single-precision%29))
  (if (not (Variables|/Game/Kaylen/Zones/BP_Zone1.BP_Zone1_C|GetIsRestored (Variables|Default|GetZone1Ref)))
    (Variables|Default|SetGiantHappiness (Math|Float|Clamp(Float) (- (Variables|Default|GetGiantHappiness) (Variables|Default|GetHappinessTickRate)) 0.0 (Variables|Default|GetGiantMaxHappiness)))
    (Default|UpdateHappinessBar (Variables|Default|GetHUDRef) self)))

(event EventBeginPlay
  (bind _returnvalue (UserInterface|CreateWidget "/Game/Kaylen/UIElements/WBP_HUD.WBP_HUD_C"))
  (bind _output_get (Variables|Default|SetHUDRef _returnvalue))
  (UserInterface|Viewport|AddtoViewport _output_get 0)
  (Default|UpdateHappinessBar (Variables|Default|GetHUDRef) self)
  (bind _outactors (Actor|GetAllActorswithTag "Fragment"))
  (Variables|Default|SetFragments _outactors))

(fn ConstructionScript)